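; Sliding door level actor that starts open and shuts once when something enters any of its trigger volumes.
; BeginPlay calls OpenDoor, and three box overlaps share a single DoOnce that calls CloseDoor, with no reset or reopen trigger wired.
; Both events check the DoorOpen flag, slide the Door vertically with MoveComponentTo, and switch the front and back light boxes between green and red glow materials.
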(event OnComponentBeginOverlap(BoxCollision)
  (params (OverlappedComponent :type Primitive%20Component%20Object%20Reference) (OtherActor :type Actor%20Object%20Reference) (OtherComp :type Primitive%20Component%20Object%20Reference) (OtherBodyIndex :type Integer) (bFromSweep :type Boolean) (SweepResult :type Hit%20Result%20Structure%20%28by%20ref%29))
  (Utilities|FlowControl|DoOnce false
    (:Completed
      (CallFunction|CloseDoor))))

(event OnComponentBeginOverlap(BoxCollision2)
  (params (OverlappedComponent :type Primitive%20Component%20Object%20Reference) (OtherActor :type Actor%20Object%20Reference) (OtherComp :type Primitive%20Component%20Object%20Reference) (OtherBodyIndex :type Integer) (bFromSweep :type Boolean) (SweepResult :type Hit%20Result%20Structure%20%28by%20ref%29))
  (Utilities|FlowControl|DoOnce false
    (:Completed
      (CallFunction|CloseDoor))))

(event OnComponentBeginOverlap(BoxCollision1)
  (params (OverlappedComponent :type Primitive%20Component%20Object%20Reference) (OtherActor :type Actor%20Object%20Reference) (OtherComp :type Primitive%20Component%20Object%20Reference) (OtherBodyIndex :type Integer) (bFromSweep :type Boolean) (SweepResult :type Hit%20Result%20Structure%20%28by%20ref%29))
  (Utilities|FlowControl|DoOnce false
    (:Completed
      (CallFunction|CloseDoor))))

(event Custom|Open%20Door
  (if (== (Variables|Default|GetDoorOpen?) false)
    (Rendering|Material|SetMaterial (Variables|Default|GetFront%20Light%20Box) 0 "/Game/LevelAssets/Materials/M_GlowGreen.M_GlowGreen")
    (Components|MoveComponentTo (Variables|Default|GetDoor) "0.000000,0.000000,-700.000000" "0, 0, 0" false false 0.2 false)
    (Variables|Default|SetDoorOpen? true)))

(event Custom|Close%20Door
  (if (Variables|Default|GetDoorOpen?)
    (Rendering|Material|SetMaterial (Variables|Default|GetFront%20Light%20Box) 0 "/Game/LevelAssets/Materials/M_GlowRed.M_GlowRed")
    (Components|MoveComponentTo (Variables|Default|GetDoor) "0.000000,0.000000,650.000000" "0, 0, 0" false false 0.2 false)
    (Variables|Default|SetDoorOpen? false)))

(event EventBeginPlay
  (CallFunction|OpenDoor))

(event Collision|EventActorBeginOverlap
  (params (OtherActor :type Actor%20Object%20Reference)))

(event EventTick
  (params (DeltaSeconds :type Float%20%28single-precision%29)))

(fn ConstructionScript)
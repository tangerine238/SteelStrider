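; BP_DialogueTrigger_Backup is a trigger actor that starts a dialogue when the third-person character overlaps it.
; It creates a HUD_Dialogue widget, passes it the dialogue DataTable and delay between lines, adds it to the viewport and calls StartDialogue.
; A DoOnce precedes the character cast, so the first overlap by any actor uses up the trigger.
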(event Collision|EventActorBeginOverlap
  (params (OtherActor :type Actor%20Object%20Reference))
  (Utilities|FlowControl|DoOnce false
    (:Completed
      (Utilities|Casting|CastToBP_ThirdPersonCharacter OtherActor)
      (bind _returnvalue (UserInterface|CreateWidget "/Game/DialogueSystem/BP/HUD/HUD_Dialogue.HUD_Dialogue_C"))
      (bind _output_get (Variables|Default|SetHUD%20Dialogue%20Ref _returnvalue))
      (Variables|/Game/DialogueSystem/BP/HUD/HUD_Dialogue.HUD_Dialogue_C|SetDialogue%20Data%20Table _output_get (Variables|Default|GetDialogue%20Data%20Table))
      (Variables|/Game/DialogueSystem/BP/HUD/HUD_Dialogue.HUD_Dialogue_C|SetDelay%20Between%20Lines _output_get (Variables|Default|GetDelay%20Between%20Lines))
      (UserInterface|Viewport|AddtoViewport _output_get 0)
      (Default|StartDialogue (Variables|Default|GetHUD%20Dialogue%20Ref)))))

(event EventTick
  (params (DeltaSeconds :type Float%20%28single-precision%29)))

(fn ConstructionScript)